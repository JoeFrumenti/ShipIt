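; BP_Player is the player Blueprint, handling movement on the world X and Y axes from Up, Down, Left and Right input actions.
; Input events set pressed flags that Tick turns into AddMovementInput, with Up and Left winning over their opposites.
; SetMovement toggles the CanMove gate.
; An UpdateControllerRotation event mirrors actor X scale by Y velocity sign, but its only call in this graph is disconnected.
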(event `UpdateMovement`
  ;[1 1 1] Movement (yes I know theres a better way to do this pls be nice)
  (if (`self.canMove`)
    (if (`self.UpPressed`)
      (set `self.XDirection` 1.0)
      (elif (`self.DownPressed`)
        (set `self.XDirection` -1.0)
        (else
          (set `self.XDirection` 0.0))))
    (if (`self.LeftPressed`)
      (set `self.YDirection` -1.0)
      (elif (`self.RightPressed`)
        (set `self.YDirection` 1.0)
        (else
          (set `self.YDirection` 0.0))))
    (`self.AddMovementInput` (`KismetMathLibrary.MakeVector` (`self.XDirection`) (`self.YDirection`)))
    (else
      (set `self.XDirection` 0.0)
      (set `self.YDirection` 0.0))))

(event `self.ReceiveTick`
  (params (DeltaSeconds :type "Float (single-precision)"))
  (`self.UpdateMovement`))

(event `InputAction|Right`
  (params (Key :type "Key Structure"))
  ;[1 1 1] Movement (yes I know theres a better way to do this pls be nice)
  (:`Pressed`
    (set `self.RightPressed` true))
  (:`Released`
    (set `self.RightPressed` false)))

(event `InputAction|Left`
  (params (Key :type "Key Structure"))
  ;[1 1 1] Movement (yes I know theres a better way to do this pls be nice)
  (:`Pressed`
    (set `self.LeftPressed` true))
  (:`Released`
    (set `self.LeftPressed` false)))

(event `InputAction|Down`
  (params (Key :type "Key Structure"))
  ;[1 1 1] Movement (yes I know theres a better way to do this pls be nice)
  (:`Pressed`
    (set `self.DownPressed` true))
  (:`Released`
    (set `self.DownPressed` false)))

(event `InputAction|Up`
  (params (Key :type "Key Structure"))
  ;[1 1 1] Movement (yes I know theres a better way to do this pls be nice)
  (:`Pressed`
    (set `self.UpPressed` true))
  (:`Released`
    (set `self.UpPressed` false)))

(event `SetMovement`
  (params (NewParam :type Boolean))
  (set `self.canMove` NewParam))

(event `UpdateControllerRotation`
  (bind _y (.y (`self.GetVelocity`)))
  ;[1 1 1] Flip direction
  (`|ExecutionSequence`
    (:`then_0`
      (if (< _y 0.0)
        (set `self.Flip` -1.0)
        (elif (> _y 0.0)
          (set `self.Flip` 1.0))))
    (:`then_1`
      (`self.SetActorScale3D` (`KismetMathLibrary.MakeVector` (`self.Flip`) 1.0 1.0)))))

(fn `UserConstructionScript`)