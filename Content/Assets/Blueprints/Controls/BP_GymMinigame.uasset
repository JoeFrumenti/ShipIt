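; BP_GymMinigame is a gym minigame Blueprint that currently resolves on debug-style key presses: W wins and L loses.
; Win and Lose each find the first top-level BP_Dialogue widget and call its CallUnloadMinigame with true or false, handing the result back to the dialogue UI.
; BeginPlay, overlap, Tick and the construction script are empty, so no other gameplay logic exists in this Blueprint.
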(event `Key|L`
  (params (Key :type "Key Structure"))
  (:`Pressed`
    (`self.Lose`)))

(event `Key|W`
  (params (Key :type "Key Structure"))
  (:`Pressed`
    (`self.Win`)))

(fn `Lose`
  (bind _foundwidgets (`WidgetBlueprintLibrary.GetAllWidgetsOfClass` "/Game/Assets/Blueprints/UI/Dialogue/BP_Dialogue.BP_Dialogue_C"))
  (`/Game/Assets/Blueprints/UI/Dialogue/BP_Dialogue.CallUnloadMinigame` (`|GetArrayItem` _foundwidgets) false))

(fn `UserConstructionScript`)

(fn `Win`
  (bind _foundwidgets (`WidgetBlueprintLibrary.GetAllWidgetsOfClass` "/Game/Assets/Blueprints/UI/Dialogue/BP_Dialogue.BP_Dialogue_C"))
  (`/Game/Assets/Blueprints/UI/Dialogue/BP_Dialogue.CallUnloadMinigame` (`|GetArrayItem` _foundwidgets) true))