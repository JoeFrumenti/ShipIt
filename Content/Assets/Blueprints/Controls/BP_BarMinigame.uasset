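; Player-controlled flipbook character for the bar minigame, which is won or lost through WinBox and LoseBox overlaps.
; Directional input actions set pressed flags that Tick turns into movement input while CanMove is true, switching between idle and walk flipbooks by velocity.
; Win and Lose report the result by calling CallUnloadMinigame on the first top-level BP_Dialogue widget found.
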(event `Key|L`
  (params (Key :type "Key Structure")))

(event `self.loseBox.OnActorBeginOverlap`
  (params (OverlappedActor :type "Actor Object Reference") (OtherActor :type "Actor Object Reference"))
  (`self.Lose`))

(event `self.winBox.OnActorBeginOverlap`
  (params (OverlappedActor :type "Actor Object Reference") (OtherActor :type "Actor Object Reference"))
  (`self.Win`))

(event `Key|W`
  (params (Key :type "Key Structure")))

(event `UpdateMovement`
  ;[1 1 1] Movement (yes I know theres a better way to do this pls be nice)
  (if (`self.canMove`)
    (if (`self.LeftPressed`)
      (set `self.XDirection` -1.0)
      (elif (`self.RightPressed`)
        (set `self.XDirection` 1.0)
        (else
          (set `self.XDirection` 0.0))))
    (if (`self.UpPressed`)
      (set `self.YDirection` 1.0)
      (elif (`self.DownPressed`)
        (set `self.YDirection` -1.0)
        (else
          (set `self.YDirection` 0.0))))
    (`self.AddMovementInput` (`KismetMathLibrary.MakeVector` (`self.YDirection`) (`self.XDirection`)))
    (if (== (`CharacterMovementComponent.GetLastUpdateVelocity` (`self.CharacterMovement`)) (0.0 0.0 0.0))
      (`PaperFlipbookComponent.SetFlipbook` (`self.Sprite`) "/Game/Assets/Sprites/mc/mc_idle/MC_idle1.MC_idle1")
      (else
        (`PaperFlipbookComponent.SetFlipbook` (`self.Sprite`) "/Game/Assets/Sprites/mc/mc_walk/mc_walk1.mc_walk1")))
    (else
      (set `self.XDirection` 0.0)
      (set `self.YDirection` 0.0))))

(event `self.ReceiveTick`
  (params (DeltaSeconds :type "Float (single-precision)"))
  (`self.UpdateMovement`))

(event `InputAction|Right`
  (params (Key :type "Key Structure"))
  ;[1 1 1] Movement (yes I know theres a better way to do this pls be nice)
  (:`Pressed`
    (set `self.RightPressed` true))
  (:`Released`
    (set `self.RightPressed` false)))

(event `InputAction|Left`
  (params (Key :type "Key Structure"))
  ;[1 1 1] Movement (yes I know theres a better way to do this pls be nice)
  (:`Pressed`
    (set `self.LeftPressed` true))
  (:`Released`
    (set `self.LeftPressed` false)))

(event `InputAction|Down`
  (params (Key :type "Key Structure"))
  ;[1 1 1] Movement (yes I know theres a better way to do this pls be nice)
  (:`Pressed`
    (set `self.DownPressed` true))
  (:`Released`
    (set `self.DownPressed` false)))

(event `InputAction|Up`
  (params (Key :type "Key Structure"))
  ;[1 1 1] Movement (yes I know theres a better way to do this pls be nice)
  (:`Pressed`
    (set `self.UpPressed` true))
  (:`Released`
    (set `self.UpPressed` false)))

(fn `Lose`
  (bind _foundwidgets (`WidgetBlueprintLibrary.GetAllWidgetsOfClass` "/Game/Assets/Blueprints/UI/Dialogue/BP_Dialogue.BP_Dialogue_C"))
  (`/Game/Assets/Blueprints/UI/Dialogue/BP_Dialogue.CallUnloadMinigame` (`|GetArrayItem` _foundwidgets) false))

(fn `NewFunction`)

(fn `UserConstructionScript`)

(fn `Win`
  (bind _foundwidgets (`WidgetBlueprintLibrary.GetAllWidgetsOfClass` "/Game/Assets/Blueprints/UI/Dialogue/BP_Dialogue.BP_Dialogue_C"))
  (`/Game/Assets/Blueprints/UI/Dialogue/BP_Dialogue.CallUnloadMinigame` (`|GetArrayItem` _foundwidgets) true))