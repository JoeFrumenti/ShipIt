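; BP_RavenMinigame is the player-controlled pawn for a raven minigame, moving in the vertical Y-Z plane.
; Up, Down, Left and Right input actions set pressed flags, which UpdateMovement reads every Tick to build a direction for AddMovementInput.
; Up and Left take priority over their opposites, and the XDirection variable drives world Z despite its name.
; A CanMove flag gates movement and zeroes both directions when false.
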(event `UpdateMovement`
  ;[1 1 1] Movement (yes I know theres a better way to do this pls be nice)
  (if (`self.canMove`)
    (if (`self.UpPressed`)
      (set `self.XDirection` 1.0)
      (elif (`self.DownPressed`)
        (set `self.XDirection` -1.0)
        (else
          (set `self.XDirection` 0.0))))
    (if (`self.LeftPressed`)
      (set `self.YDirection` -1.0)
      (elif (`self.RightPressed`)
        (set `self.YDirection` 1.0)
        (else
          (set `self.YDirection` 0.0))))
    (`self.AddMovementInput` (`KismetMathLibrary.MakeVector` 0.0 (`self.YDirection`) (`self.XDirection`)))
    (else
      (set `self.XDirection` 0.0)
      (set `self.YDirection` 0.0))))

(event `self.ReceiveTick`
  (params (DeltaSeconds :type "Float (single-precision)"))
  (`self.UpdateMovement`))

(event `InputAction|Right`
  (params (Key :type "Key Structure"))
  ;[1 1 1] Movement (yes I know theres a better way to do this pls be nice)
  (:`Pressed`
    (set `self.RightPressed` true))
  (:`Released`
    (set `self.RightPressed` false)))

(event `InputAction|Left`
  (params (Key :type "Key Structure"))
  ;[1 1 1] Movement (yes I know theres a better way to do this pls be nice)
  (:`Pressed`
    (set `self.LeftPressed` true))
  (:`Released`
    (set `self.LeftPressed` false)))

(event `InputAction|Down`
  (params (Key :type "Key Structure"))
  ;[1 1 1] Movement (yes I know theres a better way to do this pls be nice)
  (:`Pressed`
    (set `self.DownPressed` true))
  (:`Released`
    (set `self.DownPressed` false)))

(event `InputAction|Up`
  (params (Key :type "Key Structure"))
  ;[1 1 1] Movement (yes I know theres a better way to do this pls be nice)
  (:`Pressed`
    (set `self.UpPressed` true))
  (:`Released`
    (set `self.UpPressed` false)))

(fn `NewFunction`)

(fn `UserConstructionScript`)