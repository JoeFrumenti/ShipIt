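; Raven NPC Blueprint that sets up its dialogue entry point when play begins.
; On BeginPlay it finds the BP_DialogueStorage actor and copies its RavenStarter into Stats.StartNode.
; It then calls SetImage, which, despite its name, sets the Delay on top-level WB_ConversationPrompt widgets that exist at that moment.
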(event `self.ReceiveBeginPlay`
  (bind _returnvalue (`GameplayStatics.GetActorOfClass` "/Game/Assets/Blueprints/UI/Dialogue/BP_DialogueStorage.BP_DialogueStorage_C"))
  (bind _output_get (set `self.DialogueStorage` _returnvalue))
  (set `/Game/Assets/Blueprints/NPC/AC_Stats.StartNode` (`/Game/Assets/Blueprints/UI/Dialogue/BP_DialogueStorage.RavenStarter` _output_get) (`self.Stats`))
  (`self.setImage` 10.0))

(fn `setImage`
  (params (delayValue :type "Float (double-precision)"))
  (bind _foundwidgets (`WidgetBlueprintLibrary.GetAllWidgetsOfClass` "/Game/UI/WB_ConversationPrompt.WB_ConversationPrompt_C"))
  (for _array_element _foundwidgets
    (bind _aswb_conversation_prompt (cast `/Game/UI/WB_ConversationPrompt` _array_element))
    (set `/Game/UI/WB_ConversationPrompt.delay` delayValue _aswb_conversation_prompt)))

(fn `UserConstructionScript`)